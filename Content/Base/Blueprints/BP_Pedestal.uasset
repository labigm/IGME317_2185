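; BP_Pedestal is a display actor that shows a configurable skeletal mesh with a text label.
; The construction script assigns the mesh and text, shifts the mesh by a world-space offset, and scales it by the product of an individual and a general scale.
; On BeginPlay, the mesh plays its chosen animation on a loop.
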(event EventBeginPlay
  (Components|Animation|PlayAnimation (Variables|Default|GetSkeletalMesh) (Variables|Default|GetAnimationToPlay) true))

(fn ConstructionScript
  (Class|SkinnedMeshComponent|SetSkeletalMesh (Variables|Default|GetSkeletalMesh) (Variables|Default|GetSkeletonToDisplay) true)
  (Rendering|Components|TextRender|SetText (Variables|Default|GetTextRender) (Variables|Default|GetText))
  (Transformation|SetWorldLocation (Variables|Default|GetSkeletalMesh) (+ (Transformation|GetWorldLocation (Variables|Default|GetSkeletalMesh)) (Variables|Default|GetOffset)) false false)
  (Transformation|SetRelativeScale3D (Variables|Default|GetSkeletalMesh) (* (Variables|Default|GetScaleIndividual) (Variables|Default|GetScale))))
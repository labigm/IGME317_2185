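; BP_Dolgos_TP is a playable character, likely third-person, that lets the player body-hop into other characters by touch.
; Axis and action inputs drive yaw-relative movement, controller look and jumping.
; When the player-controlled instance's Transfer component overlaps a BPI_Character actor, the player controller possesses that pawn and this one spawns a default controller.
; A two-second delay after possession arms the next transfer; unpossession disarms it.
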(event OnComponentBeginOverlap(Transfer)
  (params (OverlappedComponent :type Primitive%20Component%20Object%20Reference) (OtherActor :type Actor%20Object%20Reference) (OtherComp :type Primitive%20Component%20Object%20Reference) (OtherBodyIndex :type Integer) (bFromSweep :type Boolean) (SweepResult :type Hit%20Result%20Structure%20%28by%20ref%29))
  ;[1 1 1] Check if instance is currently controlled by player
  (if (== (Pawn|GetController) (Game|GetPlayerController 0))
    ;[1 1 1] Check if ready to possess and if interface is implemented; if so, posses the colliding actor and generate new controller
    (if (Variables|Default|GetReadyToPossess?)
      (if (Utilities|DoesObjectImplementInterface OtherActor "/Game/General/BPI_Character.BPI_Character_C")
        (bind _aspawn (Utilities|Casting|CastToPawn OtherActor))
        (Pawn|Possess (Game|GetPlayerController 0) _aspawn)
        (Pawn|SpawnDefaultController)))))

(event EventPossessed
  (params (NewController :type Controller%20Object%20Reference))
  ;[1 1 1] When the character is possessed wait for a bit before letting it posses something else
  (Utilities|FlowControl|Delay 2.0)
  (Variables|Default|SetReadyToPossess? true))

(event EventUnpossessed
  (params (OldController :type Controller%20Object%20Reference))
  ;[1 1 1] When the character is possessed wait for a bit before letting it posses something else
  (Variables|Default|SetReadyToPossess? false))

(event Input|ActionEvents|InputActionJump
  (params (Key :type Key%20Structure))
  (:Pressed
    (Character|Jump)))

(event Input|AxisEvents|InputAxisMoveForward
  (params (AxisValue :type Float%20%28single-precision%29))
  (Pawn|Input|AddMovementInput (Math|Vector|GetForwardVector (Math|Rotator|MakeRotator 0.0 0.0 (.Yaw (Math|Rotator|BreakRotator (Pawn|GetControlRotation :!class /Script/Engine.Pawn))))) AxisValue false))

(event Input|AxisEvents|InputAxisMoveRight
  (params (AxisValue :type Float%20%28single-precision%29))
  (Pawn|Input|AddMovementInput (Math|Vector|GetRightVector (Math|Rotator|MakeRotator 0.0 0.0 (.Yaw (Math|Rotator|BreakRotator (Pawn|GetControlRotation :!class /Script/Engine.Pawn))))) AxisValue false))

(event Input|AxisEvents|InputAxisTurn
  (params (AxisValue :type Float%20%28single-precision%29))
  (Pawn|Input|AddControllerYawInput AxisValue))

(event Input|AxisEvents|InputAxisLookUp
  (params (AxisValue :type Float%20%28single-precision%29))
  (Pawn|Input|AddControllerPitchInput AxisValue))

(fn ConstructionScript)